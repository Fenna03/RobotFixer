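; BP_Item is an interactable world pickup that adds a "Box" item to the player's inventory.
; Overlapping its Box component shows a CanInteract prompt widget, and ending the overlap clears it by removing all widgets from the screen.
; On Interact, it sends AddItemMessage to the player character, adds the hardcoded item to that BP_ThirdPersonCharacter's InventoryWidget, then destroys itself.
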(event `/Game/extras/BPI_Interact.Interact`
  (message `/Game/extras/BP_UI.AddItem` (`GameplayStatics.GetPlayerCharacter` 0) self)
  (bind _asbp_third_person_character (cast `/Game/ThirdPerson/Blueprints/BP_ThirdPersonCharacter` (`GameplayStatics.GetPlayerCharacter` 0)))
  (`/Game/extras/WB_Inventory.AddItemToUI` (`/Game/ThirdPerson/Blueprints/BP_ThirdPersonCharacter.InventoryWidget` _asbp_third_person_character) "Box" 1)
  (`self.K2_DestroyActor`))

(event `self.Box.OnComponentBeginOverlap`
  (params (OverlappedComponent :type "PrimitiveComponent Object Reference") (OtherActor :type "Actor Object Reference") (OtherComp :type "PrimitiveComponent Object Reference") (OtherBodyIndex :type Integer) (bFromSweep :type Boolean) (SweepResult :type "HitResult Structure (by ref)"))
  (bind _returnvalue (`|CreateWidget` "/Game/extras/CanInteract.CanInteract_C"))
  (`UserWidget.AddToViewport` _returnvalue 0))

(event `self.Box.OnComponentEndOverlap`
  (params (OverlappedComponent :type "PrimitiveComponent Object Reference") (OtherActor :type "Actor Object Reference") (OtherComp :type "PrimitiveComponent Object Reference") (OtherBodyIndex :type Integer))
  (`WidgetLayoutLibrary.RemoveAllWidgets`))

(fn `UserConstructionScript`)