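; Test NPC actor that takes Box items from the player's inventory when interacted with.
; Interact scans the entry widgets in the player's inventory UI, reading item state from displayed text, and removes one "Box" per name containing that word.
; Overlapping its Box component shows a CanInteract prompt, and ending the overlap calls RemoveAllWidgets rather than removing just that prompt.
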(event `/Game/extras/BPI_Interact.Interact`
  (bind _asbp_third_person_character (cast `/Game/ThirdPerson/Blueprints/BP_ThirdPersonCharacter` (`GameplayStatics.GetPlayerCharacter` 0)))
  (bind _inventorywidget (`/Game/ThirdPerson/Blueprints/BP_ThirdPersonCharacter.InventoryWidget` _asbp_third_person_character))
  (bind _aswb_inventory (cast `/Game/extras/WB_Inventory` _inventorywidget))
  (`|CreateWidget` "/Game/extras/WBP_ItemEntry.WBP_ItemEntry_C" (`GameplayStatics.GetPlayerController` 0))
  (bind _verticalbox_80 (`/Game/extras/WB_Inventory.VerticalBox_80` _aswb_inventory))
  (for _index (range (+ (`PanelWidget.GetChildrenCount` _verticalbox_80) 1))
    (bind _aswbp_item_entry (cast `/Game/extras/WBP_ItemEntry` (`PanelWidget.GetChildAt` _verticalbox_80 _index)))
    (if (`KismetStringLibrary.Contains` (`KismetTextLibrary.Conv_TextToString` (`TextBlock.Text` (`/Game/extras/WBP_ItemEntry.ItemNameText` _aswbp_item_entry))) "Box")
      (`/Game/extras/WB_Inventory.RemoveItemFromUI` _inventorywidget "Box" 1))))

(event `self.Box.OnComponentBeginOverlap`
  (params (OverlappedComponent :type "PrimitiveComponent Object Reference") (OtherActor :type "Actor Object Reference") (OtherComp :type "PrimitiveComponent Object Reference") (OtherBodyIndex :type Integer) (bFromSweep :type Boolean) (SweepResult :type "HitResult Structure (by ref)"))
  (bind _returnvalue (`|CreateWidget` "/Game/extras/CanInteract.CanInteract_C"))
  (`UserWidget.AddToViewport` _returnvalue 0))

(event `self.Box.OnComponentEndOverlap`
  (params (OverlappedComponent :type "PrimitiveComponent Object Reference") (OtherActor :type "Actor Object Reference") (OtherComp :type "PrimitiveComponent Object Reference") (OtherBodyIndex :type Integer))
  (`WidgetLayoutLibrary.RemoveAllWidgets`))

(fn `UserConstructionScript`)